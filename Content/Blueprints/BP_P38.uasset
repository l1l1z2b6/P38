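; BP_P38 is a P-38 plane actor that flies itself at a fixed speed with spinning propellers.
; Each Tick, two helper functions roll the Left and Right components by their own speed variables, scaled by delta time.
; Tick then applies an unswept world offset from a float converted to a vector, so movement runs equally along X, Y and Z, regardless of facing.
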(event `self.ReceiveTick`
  (params (DeltaSeconds :type "Float (single-precision)"))
  (`self.NewFunction_0`)
  (`self.NewFunction_1`)
  (`self.K2_AddActorWorldOffset` (`KismetMathLibrary.Conv_DoubleToVector` (* (`GameplayStatics.GetWorldDeltaSeconds`) 200.0))))

(fn `NewFunction_0`
  (`SceneComponent.K2_AddLocalRotation` (`self.Left`) (`KismetMathLibrary.MakeRotator` (* (`GameplayStatics.GetWorldDeltaSeconds`) (`self.PropellerRotateSpeed_L`))) false false))

(fn `NewFunction_1`
  (`SceneComponent.K2_AddLocalRotation` (`self.Right`) (`KismetMathLibrary.MakeRotator` (* (`GameplayStatics.GetWorldDeltaSeconds`) (`self.PropellerRotateSpeed_R`))) false false))

(fn `UserConstructionScript`)