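; Player-controlled P-38 aircraft pawn that constantly flies forward and steers with roll and pitch input.
; Each tick spins the left and right propellers at their own speed variables, then adds forward movement input along the actor's facing.
; Roll and Pitch axes apply delta-time-scaled local rotation to the whole actor.
; An unconnected local-offset movement node remains in the event graph and never runs.
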(event `self.ReceiveTick`
  (params (DeltaSeconds :type "Float (single-precision)"))
  (`|ExecutionSequence`
    (:`then_0`
      (`self.NewFunction_0`))
    (:`then_1`
      (`self.NewFunction_1`))
    (:`then_2`
      (`self.AddMovementInput` (`self.GetActorForwardVector`)))))

(event `InputAxis|Roll`
  (params (AxisValue :type "Float (single-precision)"))
  (`self.K2_AddActorLocalRotation` (`KismetMathLibrary.MakeRotator` (* AxisValue 60.0 (`GameplayStatics.GetWorldDeltaSeconds`)))))

(event `InputAxis|Pitch`
  (params (AxisValue :type "Float (single-precision)"))
  (`self.K2_AddActorLocalRotation` (`KismetMathLibrary.MakeRotator` 0.0 (* AxisValue 60.0 (`GameplayStatics.GetWorldDeltaSeconds`)))))

(fn `NewFunction_0`
  (`SceneComponent.K2_AddLocalRotation` (`self.Left`) (`KismetMathLibrary.MakeRotator` (* (`GameplayStatics.GetWorldDeltaSeconds`) (`self.PropellerRotateSpeed_L`))) false false))

(fn `NewFunction_1`
  (`SceneComponent.K2_AddLocalRotation` (`self.Right`) (`KismetMathLibrary.MakeRotator` (* (`GameplayStatics.GetWorldDeltaSeconds`) (`self.PropellerRotateSpeed_R`))) false false))

(fn `UserConstructionScript`)